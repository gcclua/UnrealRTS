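; PlayerVitals tracks the player's health and wood, stone and metal totals, and also bootstraps the core gameplay systems.
; BeginPlay creates the HUD, minimap and mouse-interaction widgets, spawns the unit and entity managers, cross-wires them, and switches the view to the placed CameraMovementBP.
; Gather events add resources, while enemies reaching the end are destroyed and subtract health, each updating the HUD.
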(event EventOnEnemyReachEnd
  (params (enemyActor :type Actor%20Object%20Reference) (enemyType :type EnemyType%20Enum :default "Default") (damage :type Float%20%28double-precision%29))
  (bind _asenemy_base (Utilities|Casting|CastToEnemyBase enemyActor)
    (:then
      (Class|CharacterEntityBase|OnDestroy _asenemy_base))
    (:CastFailed
      _))
  (Actor|DestroyActor enemyActor)
  (if (<= (- (Variables|Default|GetHealth) damage) 0.0)
    (Variables|Default|SetHealth 0.0))
  (bind _output_get (Variables|Default|SetHealth (- (Variables|Default|GetHealth) damage)))
  (Default|SetHealth (Variables|Default|GetHUD) _output_get))

(event EventOnGatherResource
  (params (resource :type ResourceType%20Enum :default "Wood") (amount :type Integer))
  (switch Utilities|FlowControl|Switch|SwitchonResourceType resource
    (:Wood
      ;[0 0 0] Wood
      (bind _output_get (Variables|Default|SetWood (+ (Variables|Default|GetWood) amount)))
      (Default|SetWood (Variables|Default|GetHUD) _output_get))
    (:Stone
      ;[0 0 0] Stone
      (bind _output_get_2 (Variables|Default|SetStone (+ amount (Variables|Default|GetStone))))
      (Default|SetStone (Variables|Default|GetHUD) _output_get_2))
    (:Metal
      ;[0 0 0] Metal
      (bind _output_get_3 (Variables|Default|SetMetal (+ amount (Variables|Default|GetMetal))))
      (Default|SetMetal (Variables|Default|GetHUD) _output_get_3))))

(event Custom|SetupVariables
  (Variables|Default|SetMetal 0)
  (Variables|Default|SetWood 0)
  (Variables|Default|SetStone 0)
  (bind _output_get (Variables|Default|SetHealth (Variables|Default|GetStartingHealth)))
  (Default|SetHealth (Variables|Default|GetHUD) _output_get))

(event EventBeginPlay
  (bind _returnvalue (Game|GetPlayerController 0))
  (bind _returnvalue_2 (Transformation|GetActorTransform))
  (bind _returnvalue_3 (UserInterface|CreateWidget "/Game/Blueprints/UI/PlayerHUD.PlayerHUD_C"))
  (bind _output_get (Variables|Default|SetHUD _returnvalue_3))
  (Class|HUDBase|Setup _output_get _returnvalue)
  (UserInterface|Viewport|AddtoViewport _output_get 0)
  (CallFunction|SetupVariables)
  (bind _returnvalue_4 (UserInterface|CreateWidget "/Game/Blueprints/UI/MiniMapBP.MiniMapBP_C"))
  (bind _returnvalue_5 (Actor|GetActorOfClass "/Game/Blueprints/Core/CameraMovementBP.CameraMovementBP_C"))
  (Class|MiniMap|Setup _returnvalue_4 _returnvalue _returnvalue_5)
  (UserInterface|Viewport|AddtoViewport _returnvalue_4 0)
  (bind _returnvalue_6 (UserInterface|CreateWidget "/Game/Blueprints/UI/MouseInteraction.MouseInteraction_C"))
  (UserInterface|Viewport|AddtoViewport _returnvalue_6 0)
  (bind _returnvalue_7 (Game|SpawnActorfromClass "/Script/TowerDefense.UnitManager" _returnvalue_2 "Undefined" "MultiplyWithRoot" 0 0))
  (Class|UnitManager|Setup _returnvalue_7 _output_get _returnvalue_6 _returnvalue)
  (bind _returnvalue_8 (Game|SpawnActorfromClass "/Script/TowerDefense.EntityManager" _returnvalue_2 "Undefined" "OverrideRootScale" 0 0))
  (Class|EntityManager|Setup _returnvalue_8 _returnvalue_4 _returnvalue_6 _returnvalue_7)
  (Class|MouseInteractionBase|Setup _returnvalue_6 _returnvalue _returnvalue_8)
  (Class|CameraMovement|Setup _returnvalue_5 _returnvalue _returnvalue_6)
  (Game|Player|SetViewTargetwithBlend _returnvalue _returnvalue_5 0.0 "VTBlend_Linear" 0.0 false))

(fn ConstructionScript)