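; Enemy spawner actor that spawns a wave of AI enemies at its own location, starting on BeginPlay.
; A self-calling SpawnEnemy event spawns one enemy every few seconds, incrementing CurrentAmount until it equals MaxAmount.
; After the final spawn and a longer delay, it finds an EnemySpawner1 actor and sets its Start flag to chain to that spawner.
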(event Custom|SpawnEnemy
  (AI|SpawnAIFromClass "/Game/Blueprints/Enemy.Enemy_C" 0 (Transformation|GetActorLocation) "0, 0, 0" false 0)
  (if (== (Variables|Default|GetCurrentAmount) (Variables|Default|GetMaxAmount))
    (Utilities|FlowControl|Delay 3e+01)
    (bind _returnvalue (Actor|GetActorOfClass "/Game/Blueprints/EnemySpawner1.EnemySpawner1_C"))
    (Variables|/Game/Blueprints/EnemySpawner1.EnemySpawner1_C|SetStart? _returnvalue true)
    (else
      (Variables|Default|SetCurrentAmount (+ 1 (Variables|Default|GetCurrentAmount)))
      (Utilities|FlowControl|Delay 3.0)
      (CallFunction|SpawnEnemy))))

(event EventBeginPlay
  (CallFunction|SpawnEnemy))

(fn ConstructionScript)