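; TowerSpawn is a clickable tower spawn spot whose plane changes material to reflect cursor hover, click and release.
; A click that passes the Tower check turns the plane green, removes any open TowerList widgets and opens a new one.
; The new TowerList receives a reference to this spot through its TowerSpawn variable.
; A click that fails the check only turns the plane orange.
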(event OnBeginCursorOver(Plane)
  (params (TouchedComponent :type Primitive%20Component%20Object%20Reference))
  (Rendering|Material|SetMaterial (Variables|Default|GetPlane) 0 "/Game/Art/Black.Black"))

(event OnEndCursorOver(Plane)
  (params (TouchedComponent :type Primitive%20Component%20Object%20Reference))
  (Rendering|Material|SetMaterial (Variables|Default|GetPlane) 0 "/Game/Art/White.White"))

(event OnClicked(Plane)
  (params (TouchedComponent :type Primitive%20Component%20Object%20Reference) (ButtonPressed :type Key%20Structure :default "None"))
  (if (Variables|Default|GetTower?)
    (Rendering|Material|SetMaterial (Variables|Default|GetPlane) 0 "/Game/Art/Green.Green")
    (bind _foundwidgets (Widget|GetAllWidgetsOfClass "/Game/Blueprints/TowerList.TowerList_C" true))
    (for _array_element _foundwidgets
      (Widget|RemovefromParent _array_element))
    (bind _returnvalue (UserInterface|CreateWidget "/Game/Blueprints/TowerList.TowerList_C"))
    (UserInterface|Viewport|AddtoViewport _returnvalue 0)
    (Variables|/Game/Blueprints/TowerList.TowerList_C|SetTowerSpawn _returnvalue self)
    (else
      (Rendering|Material|SetMaterial (Variables|Default|GetPlane) 0 "/Game/Art/Orange.Orange"))))

(event OnReleased(Plane)
  (params (TouchedComponent :type Primitive%20Component%20Object%20Reference) (ButtonReleased :type Key%20Structure :default "None"))
  (Rendering|Material|SetMaterial (Variables|Default|GetPlane) 0 "/Game/Art/White.White"))

(event EventBeginPlay)

(event Collision|EventActorBeginOverlap
  (params (OtherActor :type Actor%20Object%20Reference)))

(event EventTick
  (params (DeltaSeconds :type Float%20%28single-precision%29)))

(fn ConstructionScript)