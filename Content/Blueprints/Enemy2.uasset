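; Enemy2 is an enemy character that walks to a Goal actor and damages the player's TowerPawn.
; On BeginPlay it waits briefly, sets its walk speed and uses AI MoveTo toward the first Goal found in the level.
; Both move success and failure subtract a fixed amount from TowerPawn health, then destroy the enemy after a delay.
; Its own Health variable is unused here.
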(event EventBeginPlay
  (Utilities|FlowControl|Delay 0.2)
  (Variables|/Script/Engine.CharacterMovementComponent|SetMaxWalkSpeed (Variables|Character|GetCharacterMovement) 2e+02)
  (bind _outactors (Actor|GetAllActorsOfClass "/Game/Blueprints/Goal.Goal_C"))
  (AI|AIMoveTo self "0, 0, 0" (Utilities|Array|Get(acopy) _outactors) 5.0 false
    (:OnSuccess
      _)
    (:OnFail
      _))
  (bind _astower_pawn (Utilities|Casting|CastToTowerPawn (Game|Player|GetPlayerPawn 0)))
  (Variables|/Game/Blueprints/TowerPawn.TowerPawn_C|SetHealth _astower_pawn (- (Variables|/Game/Blueprints/TowerPawn.TowerPawn_C|GetHealth _astower_pawn) 1e+01))
  (Utilities|FlowControl|Delay 3.0)
  (Actor|DestroyActor))

(fn ConstructionScript
  (|CallParentFunction))