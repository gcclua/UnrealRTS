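; Rocket tower that tracks enemies within range and fires rockets at them.
; RangeCollision overlaps maintain a GUID-keyed map of potential targets.
; Tick picks the closest enemy when untargeted, smoothly turns yaw toward it and fires on a real-time cooldown, keeping that target until it leaves range.
; Each spawned Rocket_BT receives the target and the EffectsManager found at BeginPlay.
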(event OnComponentBeginOverlap(RangeCollision)
  (params (OverlappedComponent :type Primitive%20Component%20Object%20Reference) (OtherActor :type Actor%20Object%20Reference) (OtherComp :type Primitive%20Component%20Object%20Reference) (OtherBodyIndex :type Integer) (bFromSweep :type Boolean) (SweepResult :type Hit%20Result%20Structure%20%28by%20ref%29))
  (bind _potentialtargets (Variables|Default|GetPotentialTargets))
  ;[0.01764 0.01764 0.01764] Add enemy to PotentialTargets when in range
  (bind _asenemy_base (Utilities|Casting|CastToEnemyBase OtherActor))
  (if (not (Utilities|Map|Contains _potentialtargets (Variables|/Script/Engine.Actor|GetActorGuid _asenemy_base)))
    (Utilities|Map|Add _potentialtargets (Variables|/Script/Engine.Actor|GetActorGuid _asenemy_base) _asenemy_base)))

(event OnComponentEndOverlap(RangeCollision)
  (params (OverlappedComponent :type Primitive%20Component%20Object%20Reference) (OtherActor :type Actor%20Object%20Reference) (OtherComp :type Primitive%20Component%20Object%20Reference) (OtherBodyIndex :type Integer))
  (bind _potentialtargets (Variables|Default|GetPotentialTargets))
  ;[0.01764 0.01764 0.01764] Remove Enemy to PotentialTargets when out of range
  (bind _asenemy_base (Utilities|Casting|CastToEnemyBase OtherActor))
  (if (Utilities|Map|Contains _potentialtargets (Variables|/Script/Engine.Actor|GetActorGuid _asenemy_base))
    (Utilities|Map|Remove _potentialtargets (Variables|/Script/Engine.Actor|GetActorGuid _asenemy_base))
    (if (Utilities|Map|IsEmpty (Variables|Default|GetPotentialTargets)) ; Set HasTarget to false if PotentialTargets is empty or the CurrentTarget equals what was just removed
      (Variables|Default|SetHasTarget false :!label _label)
      (elif (== (Variables|Default|GetCurrentTarget) _asenemy_base)
        (goto _label)))))

(event Custom|Fire
  (bind _spawnpoint (Variables|Default|GetSpawnPoint))
  ;[0.01764 0.01764 0.01764] Firing
  (Variables|Default|SetNextFireTime (+ (Utilities|Time|GetRealTimeSeconds) (Variables|Default|GetFiringSpeed)))
  (bind _returnvalue (Game|SpawnActorfromClass "/Game/Blueprints/BulletTypes/Rocket_BT.Rocket_BT_C" (Transformation|GetWorldTransform _spawnpoint) "Undefined" 0 0))
  (Transformation|SetActorRotation _returnvalue (Variables|/Script/Engine.SceneComponent|GetRelativeRotation _spawnpoint))
  (Default|Fire _returnvalue (Variables|Default|GeteffectsManager) 1 (Variables|Default|GetCurrentTarget)))

(event EventBeginPlay
  ;[0.01764 0.01764 0.01764] BeginPlay
  (Components|Sphere|SetSphereRadius (Variables|Default|GetRangeCollision) (Variables|Default|GetRange) true)
  (Variables|Default|SetNextFireTime 0.0)
  (bind _returnvalue (Actor|GetActorOfClass "/Game/Blueprints/EffectsManager.EffectsManager_C"))
  (Utilities|IsValid _returnvalue
    (:Is%20Valid
      (Development|PrintString "valid")
      (Variables|Default|SeteffectsManager _returnvalue))))

(event EventTick
  (params (DeltaSeconds :type Float%20%28single-precision%29))
  ;[0.01764 0.01764 0.01764] Main Loop
  (if (Variables|Default|GetHasTarget)
    (Utilities|IsValid (Variables|Default|GetCurrentTarget) :!label _label
      (:Is%20Valid
        (Transformation|SetActorRotation (Math|Rotator|MakeRotator 0.0 0.0 (.yaw (Math|Interpolation|RInterpTo (Transformation|GetActorRotation) (Math|Rotator|FindLookatRotation (Transformation|GetActorLocation) (Transformation|GetActorLocation (Variables|Default|GetCurrentTarget))) DeltaSeconds 2e+01))))
        (if (>= (Utilities|Time|GetRealTimeSeconds) (Variables|Default|GetNextFireTime))
          (CallFunction|Fire))))
    (else
      (CallFunction|SetClosestEnemy)
      (if (Variables|Default|GetHasTarget)
        (goto _label)))))

(fn ConstructionScript
  (|CallParentFunction))

(fn SetClosestEnemy
  (Variables|Default|SetHasTarget (Utilities|Map|IsNotEmpty (Variables|Default|GetPotentialTargets)))
  (if (Variables|Default|GetHasTarget)
    (LocalVariables|SetMinDist 999999.0)
    (bind _keys (Utilities|Map|Keys (Variables|Default|GetPotentialTargets)))
    (for _array_element _keys
      (if (< (Math|Vector|Distance(Vector) (Transformation|GetActorLocation (.Value (Utilities|Map|Find (Variables|Default|GetPotentialTargets) _array_element))) (Transformation|GetActorLocation)) (LocalVariables|GetMinDist))
        (LocalVariables|SetMinDist (Math|Vector|Distance(Vector) (Transformation|GetActorLocation (.Value (Utilities|Map|Find (Variables|Default|GetPotentialTargets) _array_element))) (Transformation|GetActorLocation)))
        (Variables|Default|SetCurrentTarget (.Value (Utilities|Map|Find (Variables|Default|GetPotentialTargets) _array_element))))))
  (return))