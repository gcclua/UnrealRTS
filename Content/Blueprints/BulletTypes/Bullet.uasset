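; Base projectile actor for bullet types, fired at a target enemy with an effects manager and projectile type.
; Fire stores those references, calls the FireFunctionality event as an overridable hook, then destroys the bullet after a timeout.
; Overlapping an EnemyBase applies a hit, plays the type's effect through the manager and destroys the bullet.
; GetTravelTime estimates flight time to a point from distance and the projectile movement's max speed.
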(event Custom|Fire
  (params (effectManager :type Effects%20Manager%20Object%20Reference) (projectileType :type Integer) (targetEnemy :type Enemy%20Base%20Object%20Reference))
  ;[1 1 1] Bullet Functionality
  ;;[1 1 1] Core Functionality
  (Variables|Default|SeteffectsManager effectManager)
  (Variables|Default|SetprojectileType projectileType)
  (Variables|Default|SettargetEnemy targetEnemy)
  (Development|PrintString "Base")
  (CallFunction|FireFunctionality)
  (Utilities|FlowControl|Delay 1e+01)
  (Actor|DestroyActor))

(event Custom|Fire%20Functionality
  ;[1 1 1] Bullet Functionality
  (Development|PrintString "Custom Fire FUnctionality"))

(event Collision|EventActorBeginOverlap
  (params (OtherActor :type Actor%20Object%20Reference))
  ;[1 1 1] Shipped
  ;;[1 1 1] Destroy On Collision
  (bind _asenemy_base (Utilities|Casting|CastToEnemyBase OtherActor))
  (Default|EnemyHit _asenemy_base 1.0)
  (Default|PlayEffect (Variables|Default|GeteffectsManager) (Transformation|GetActorTransform) (Variables|Default|GetprojectileType))
  (Actor|DestroyActor))

(fn ConstructionScript)

(fn GetTravelTime
  (params (Target :type Vector))
  (return (/ (Math|Vector|Distance(Vector) (Transformation|GetActorLocation) Target) (Class|MovementComponent|GetMaxSpeed (Variables|Default|GetProjectileMovement)))))

(fn Destroy)