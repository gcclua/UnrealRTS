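; Homing rocket projectile that chases a target enemy and damages it on contact.
; OnFire aligns the rocket to the spawn transform's rotation and turns on ProjectileMovement homing toward the target's scene component.
; Overlapping an EnemyBase calls EnemyHit, plays an effect at the rocket's position through the level's EffectsManager, then destroys the rocket.
; Overlaps with other actors only print a debug message.
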(event Custom|OnFire
  (params (TargetEnemy :type Enemy%20Base%20Object%20Reference) (SpawnTransform :type Transform))
  (bind _projectilemovement (Variables|Default|GetProjectileMovement))
  (Transformation|SetActorRotation (Math|Transform|TransformRotation SpawnTransform "0, 0, 0"))
  (Variables|/Script/Engine.ProjectileMovementComponent|SetHomingTargetComponent _projectilemovement (Variables|/Game/Blueprints/EnemyBase.EnemyBase_C|GetSceneComponent TargetEnemy))
  (Variables|/Script/Engine.ProjectileMovementComponent|SetbIsHomingProjectile _projectilemovement true))

(event Collision|EventActorBeginOverlap
  (params (OtherActor :type Actor%20Object%20Reference))
  ;[1 1 1] Destroy On Collision
  (bind _asenemy_base (Utilities|Casting|CastToEnemyBase OtherActor)
    (:then
      (Development|PrintString "Enemy hit!")
      (Default|EnemyHit _asenemy_base 1.0)
      (bind _returnvalue (Actor|GetActorOfClass "/Game/Blueprints/EffectsManager.EffectsManager_C"))
      (Default|PlayEffect _returnvalue (Transformation|GetActorTransform) 1)
      (Actor|DestroyActor))
    (:CastFailed
      (Development|PrintString "Not An Enemy"))))

(fn ConstructionScript)