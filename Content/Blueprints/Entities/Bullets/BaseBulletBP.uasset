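; Base projectile actor that damages enemies on overlap and plays an impact effect through the passed-in effects manager.
; Fire stores the manager, projectile type and target, then SetProperties maps the type to damage and effect.
; The empty FireFunctionality event, called before those properties are set, serves as a hook for custom behaviour.
; The bullet destroys itself on hitting an enemy or when its fixed lifetime expires.
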(event Custom|Fire%20Functionality
  ;[1 1 1] Shipped
  ;;[1 1 1] Custom Functionality
)

(event Custom|Fire
  (params (effectManager :type Effects%20Manager%20Object%20Reference) (projectileType :type BulletType%20Enum :default "Basic") (targetEnemy :type Enemy%20Base%20BP%20Object%20Reference))
  ;[1 1 1] Shipped
  ;;[1 1 1] Initialise
  (Variables|Default|SeteffectsManager effectManager)
  (Variables|Default|SetbulletType projectileType)
  (Variables|Default|SettargetEnemy targetEnemy)
  (Development|PrintString "Base")
  (CallFunction|SetProperties)
  (Utilities|FlowControl|Delay 1e+01)
  (Actor|DestroyActor))

(event Custom|Set%20Properties
  ;[1 1 1] Shipped
  ;;[1 1 1] Set Bullet Damage
  (CallFunction|FireFunctionality)
  (switch Utilities|FlowControl|Switch|SwitchonBulletType (Variables|Default|GetbulletType)
    (:Basic
      (Variables|Default|SetbulletDamage 1.0)
      (Variables|Default|SeteffectType "BulletImpact"))
    (:Rocket
      (Variables|Default|SetbulletDamage 5.0)
      (Variables|Default|SeteffectType "Explosion"))
    (:Debug
      (Variables|Default|SetbulletDamage 1e+01)
      (Variables|Default|SeteffectType "BulletDeflect"))))

(event Collision|EventActorBeginOverlap
  (params (OtherActor :type Actor%20Object%20Reference))
  ;[1 1 1] Shipped
  ;;[1 1 1] On Hit
  (bind _asenemy_base_bp (Utilities|Casting|CastToEnemyBaseBP OtherActor))
  (Default|EnemyHit _asenemy_base_bp (Variables|Default|GetbulletDamage))
  (Default|PlayEffect (Variables|Default|GeteffectsManager) (Transformation|GetActorTransform) (Variables|Default|GeteffectType))
  (Actor|DestroyActor))

(fn ConstructionScript)