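; Base enemy character Blueprint that walks toward a Goal actor and dies when its health runs out.
; On BeginPlay it adds a scene component, waits briefly, sets its walk speed and uses AI MoveTo toward the first Goal found in the level.
; The EnemyHit event subtracts incoming damage from Health and destroys the actor at zero or below.
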(event Custom|EnemyHit
  (params (damageDealt :type Float%20%28double-precision%29))
  (bind _health (Variables|Default|Gethealth))
  ;[1 1 1] On Hit
  (Variables|Default|SetHealth (- _health damageDealt))
  (if (<= _health 0.0)
    (Actor|DestroyActor)))

(event EventBeginPlay
  (bind _returnvalue (AddComponent|AddSceneComponent false))
  (Variables|Default|SetSceneComponent _returnvalue)
  (Utilities|FlowControl|Delay 0.2)
  (Variables|/Script/Engine.CharacterMovementComponent|SetMaxWalkSpeed (Variables|Character|GetCharacterMovement) 2e+02)
  (bind _outactors (Actor|GetAllActorsOfClass "/Game/Blueprints/Goal.Goal_C"))
  (AI|AIMoveTo self "0, 0, 0" (Utilities|Array|Get(acopy) _outactors) 5.0 false))

(fn ConstructionScript)