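; BuilderBP is a builder unit that walks to an assigned building and carries out its construction job.
; OnStartJob sets walk speed, stores the target and uses AIMoveTo, tracking state through WalkingToJob, DoingJob and Idle.
; On arrival it waits the building's BuildTime, calls OnDoneConstructing on construction sites, then notifies the BuilderManager through OnCompleteBuild.
; A failed move only logs a message.
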(event EventOnStartJob
  (params (building :type Building%20Base%20Object%20Reference))
  (Variables|/Script/Engine.CharacterMovementComponent|SetMaxWalkSpeed (Variables|Character|GetCharacterMovement) 3.5e+02)
  (bind _output_get (Variables|Default|SetCurrentBuilding building))
  ;[1 1 1] move to job
  (Variables|Default|SetCurrentState "WalkingToJob")
  (AI|AIMoveTo self "0, 0, 0" _output_get 5.0 false
    (:OnSuccess
      ;[1 1 1] do the job
      (Variables|Default|SetCurrentState "DoingJob")
      (Utilities|FlowControl|Delay (Variables|/Script/TowerDefense.BuildingBase|GetBuildTime (Variables|Default|GetCurrentBuilding)))
      (Variables|Default|SetCurrentState "Idle")
      ;[1 1 1] delete construction and spawn building if there is one
      (if (Variables|/Script/TowerDefense.BuildingBase|GetIsConstruction (Variables|Default|GetCurrentBuilding))
        (Class|BuildingBase|OnDoneConstructing (Variables|Default|GetCurrentBuilding)))
      ;[1 1 1] call back to buildermanager
      (bind _returnvalue (Actor|GetActorOfClass "/Script/TowerDefense.BuilderManager"))
      (Class|BuilderManager|OnCompleteBuild _returnvalue self))
    (:OnFail
      (Utilities|String|LogString "FAIl"))))

(fn ConstructionScript)