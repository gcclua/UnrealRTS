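; Rocket tower Blueprint that fires rocket projectiles at its current target enemy.
; Its Fire event schedules the next shot from real time plus FiringSpeed, then spawns a RocketBulletBP at the SpawnPoint transform.
; It launches the new projectile with the effects manager, the Rocket projectile type and CurrentTarget.
; Target selection and the call to Fire are not in this graph, and BeginPlay, Tick and overlap events are unused.
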(event EventBeginPlay
  (|CallParentFunction) ; This node is disabled and will not be called.\nDrag off pins to build functionality.
)

(event Collision|EventActorBeginOverlap
  (params (OtherActor :type Actor%20Object%20Reference)))

(event EventTick
  (params (DeltaSeconds :type Float%20%28single-precision%29))
  (|CallParentFunction DeltaSeconds) ; This node is disabled and will not be called.\nDrag off pins to build functionality.
)

(event EventFire
  ;[0.01764 0.01764 0.01764] Firing
  (Variables|Default|SetNextFireTime (+ (Utilities|Time|GetRealTimeSeconds) (Variables|Default|GetFiringSpeed)))
  (bind _returnvalue (Game|SpawnActorfromClass "/Game/Blueprints/Entities/Bullets/RocketBulletBP.RocketBulletBP_C" (Transformation|GetWorldTransform (Variables|Default|GetSpawnPoint)) "Undefined" 0 0))
  (Default|Fire _returnvalue (Variables|Default|GeteffectsManager) "Rocket" (Variables|Default|GetCurrentTarget)))

(fn ConstructionScript
  (|CallParentFunction))