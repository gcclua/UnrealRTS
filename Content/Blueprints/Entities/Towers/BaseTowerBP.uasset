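; Base tower Blueprint that acquires enemies within range, turns to face one and triggers firing.
; A range sphere's overlap events maintain a GUID-keyed map of potential targets, clearing the target flag when the current one leaves.
; Tick picks the closest enemy only when untargeted, interpolates yaw toward it and calls Fire once real time reaches NextFireTime.
; Fire is an empty event here, and NextFireTime is only initialized.
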(event OnComponentBeginOverlap(RangeCollision)
  (params (OverlappedComponent :type Primitive%20Component%20Object%20Reference) (OtherActor :type Actor%20Object%20Reference) (OtherComp :type Primitive%20Component%20Object%20Reference) (OtherBodyIndex :type Integer) (bFromSweep :type Boolean) (SweepResult :type Hit%20Result%20Structure%20%28by%20ref%29))
  (bind _potentialtargets (Variables|Default|GetpotentialTargets))
  ;[0.01764 0.01764 0.01764] Add enemy to PotentialTargets when in range
  (bind _asenemy_base_bp (Utilities|Casting|CastToEnemyBaseBP OtherActor))
  (if (not (Utilities|Map|Contains _potentialtargets (Variables|/Script/Engine.Actor|GetActorGuid _asenemy_base_bp)))
    (Utilities|Map|Add _potentialtargets (Variables|/Script/Engine.Actor|GetActorGuid _asenemy_base_bp) _asenemy_base_bp)))

(event OnComponentEndOverlap(RangeCollision)
  (params (OverlappedComponent :type Primitive%20Component%20Object%20Reference) (OtherActor :type Actor%20Object%20Reference) (OtherComp :type Primitive%20Component%20Object%20Reference) (OtherBodyIndex :type Integer))
  (bind _potentialtargets (Variables|Default|GetpotentialTargets))
  ;[0.01764 0.01764 0.01764] Remove Enemy to PotentialTargets when out of range
  (bind _asenemy_base_bp (Utilities|Casting|CastToEnemyBaseBP OtherActor))
  (if (Utilities|Map|Contains _potentialtargets (Variables|/Script/Engine.Actor|GetActorGuid _asenemy_base_bp))
    (Utilities|Map|Remove _potentialtargets (Variables|/Script/Engine.Actor|GetActorGuid _asenemy_base_bp))
    (if (Utilities|Map|IsEmpty _potentialtargets) ; Set HasTarget to false if PotentialTargets is empty or the CurrentTarget equals what was just removed
      (Variables|Default|SetHasTarget false :!label _label)
      (elif (== (Variables|Default|GetcurrentTarget) _asenemy_base_bp)
        (goto _label)))))

(event Custom|Fire
  ;[0.01764 0.01764 0.01764] Main Loop
  ;;[1 1 1] Fire Event
)

(event EventBeginPlay
  ;[0.01764 0.01764 0.01764] BeginPlay
  (Components|Sphere|SetSphereRadius (Variables|Default|GetRangeCollision) (Variables|Default|Getrange) true)
  (Variables|Default|SetnextFireTime 0.0)
  (bind _returnvalue (Actor|GetActorOfClass "/Game/Blueprints/EffectsManager.EffectsManager_C"))
  (Variables|Default|SeteffectsManager _returnvalue))

(event EventTick
  (params (DeltaSeconds :type Float%20%28single-precision%29))
  ;[0.01764 0.01764 0.01764] Main Loop
  (if (Variables|Default|GethasTarget)
    (Utilities|IsValid (Variables|Default|GetCurrentTarget) :!label _label
      (:Is%20Valid
        (Transformation|SetActorRotation (Math|Rotator|MakeRotator 0.0 0.0 (.yaw (Math|Interpolation|RInterpTo (Transformation|GetActorRotation) (Math|Rotator|FindLookatRotation (Transformation|GetActorLocation) (Transformation|GetActorLocation (Variables|Default|GetcurrentTarget))) DeltaSeconds 2e+01))) true)
        (if (>= (Utilities|Time|GetRealTimeSeconds) (Variables|Default|GetNextFireTime))
          (CallFunction|Fire))))
    (else
      (CallFunction|SetClosestEnemy)
      (if (Variables|Default|GethasTarget)
        (goto _label)))))

(fn ConstructionScript)

(fn SetClosestEnemy
  (bind _potentialtargets (Variables|Default|GetpotentialTargets))
  (Variables|Default|SetHasTarget (Utilities|Map|IsNotEmpty _potentialtargets))
  (if (Variables|Default|GetHasTarget)
    (LocalVariables|SetMinDist 999999.0)
    (bind _keys (Utilities|Map|Keys _potentialtargets))
    (for _array_element _keys
      (if (< (Math|Vector|Distance(Vector) (Transformation|GetActorLocation (.Value (Utilities|Map|Find _potentialtargets _array_element))) (Transformation|GetActorLocation)) (LocalVariables|GetMinDist))
        (LocalVariables|SetMinDist (Math|Vector|Distance(Vector) (Transformation|GetActorLocation (.Value (Utilities|Map|Find _potentialtargets _array_element))) (Transformation|GetActorLocation)))
        (Variables|Default|SetcurrentTarget (.Value (Utilities|Map|Find _potentialtargets _array_element))))))
  (return))