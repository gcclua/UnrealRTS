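; TowerBaseBP is the base tower Blueprint that tracks its current target and fires on a timer.
; On BeginPlay it caches the level's EffectsManager.
; Each tick with a valid target, it smoothly interpolates its yaw toward that target and calls Fire once real time passes NextFireTime.
; Fire is an empty event here, apparently left for child towers to implement.
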(event Custom|Fire
  ;[0.01764 0.01764 0.01764] Main Loop
  ;;[1 1 1] Fire Event
)

(event EventBeginPlay
  ;[0.01764 0.01764 0.01764] BeginPlay
  (bind _returnvalue (Actor|GetActorOfClass "/Game/Blueprints/Systems/EffectsManager.EffectsManager_C"))
  (Variables|Default|SeteffectsManager _returnvalue))

(event EventTick
  (params (DeltaSeconds :type Float%20%28single-precision%29))
  ;[0.01764 0.01764 0.01764] Main Loop
  (bind _returnvalue (Class|TowerBase|HasTarget))
  (if _returnvalue
    (Transformation|SetActorRotation (Math|Rotator|MakeRotator 0.0 0.0 (.yaw (Math|Interpolation|RInterpTo (Transformation|GetActorRotation) (Math|Rotator|FindLookatRotation (Transformation|GetActorLocation) (Transformation|GetActorLocation (Variables|Default|GetCurrentTarget))) DeltaSeconds 2e+01))) true)
    (if (>= (Utilities|Time|GetRealTimeSeconds) (Variables|Default|GetNextFireTime))
      (CallFunction|Fire))))

(fn ConstructionScript)