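; TowerSpawn is a clickable tower spawn spot that opens a TowerList widget.
; Its Plane swaps materials as feedback for cursor hover, click and release.
; On click, a check on Tower either turns the plane green and opens the list or just turns it orange.
; Opening the list first removes existing top-level TowerList widgets, then passes this actor to the new one as TowerSpawn.
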(event OnBeginCursorOver(Plane)
  (params (TouchedComponent :type Primitive%20Component%20Object%20Reference))
  (Rendering|Material|SetMaterial (Variables|Default|GetPlane) 0 "/Game/Art/Materials/Black.Black"))

(event OnEndCursorOver(Plane)
  (params (TouchedComponent :type Primitive%20Component%20Object%20Reference))
  (Rendering|Material|SetMaterial (Variables|Default|GetPlane) 0 "/Game/Art/Materials/White.White"))

(event OnClicked(Plane)
  (params (TouchedComponent :type Primitive%20Component%20Object%20Reference) (ButtonPressed :type Key%20Structure))
  (if (Variables|Default|GetTower?)
    (Rendering|Material|SetMaterial (Variables|Default|GetPlane) 0 "/Game/Art/Materials/Green.Green")
    (bind _foundwidgets (Widget|GetAllWidgetsOfClass "/Game/Blueprints/UI/TowerList.TowerList_C" true))
    (for _array_element _foundwidgets
      (Widget|RemovefromParent _array_element))
    (bind _returnvalue (UserInterface|CreateWidget "/Game/Blueprints/UI/TowerList.TowerList_C"))
    (UserInterface|Viewport|AddtoViewport _returnvalue 0)
    (Variables|/Game/Blueprints/UI/TowerList.TowerList_C|SetTowerSpawn _returnvalue self)
    (else
      (Rendering|Material|SetMaterial (Variables|Default|GetPlane) 0 "/Game/Art/Materials/Orange.Orange"))))

(event OnReleased(Plane)
  (params (TouchedComponent :type Primitive%20Component%20Object%20Reference) (ButtonReleased :type Key%20Structure))
  (Rendering|Material|SetMaterial (Variables|Default|GetPlane) 0 "/Game/Art/Materials/White.White"))

(event EventBeginPlay)

(event Collision|EventActorBeginOverlap
  (params (OtherActor :type Actor%20Object%20Reference)))

(event EventTick
  (params (DeltaSeconds :type Float%20%28single-precision%29)))

(fn ConstructionScript)