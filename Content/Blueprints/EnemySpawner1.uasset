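; Enemy spawner actor that spawns AI pawns of its Enemy class at its own location.
; BeginPlay triggers SpawnEnemy if the Start flag is set, then clears the flag.
; SpawnEnemy re-calls itself after a fixed delay, incrementing CurrentAmount until it equals MaxAmount.
; The limit is checked after each spawn, so a count starting at zero yields one enemy more than MaxAmount.
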(event Custom|SpawnEnemy
  (AI|SpawnAIFromClass "/Game/Blueprints/Enemy.Enemy_C" 0 (Transformation|GetActorLocation) "0, 0, 0" false 0)
  (if (not (== (Variables|Default|GetCurrentAmount) (Variables|Default|GetMaxAmount)))
    (Variables|Default|SetCurrentAmount (+ 1 (Variables|Default|GetCurrentAmount)))
    (Utilities|FlowControl|Delay 3.0)
    (CallFunction|SpawnEnemy)))

(event EventBeginPlay
  (if (Variables|Default|GetStart?)
    (CallFunction|SpawnEnemy)
    (Variables|Default|SetStart? false)))

(fn ConstructionScript)